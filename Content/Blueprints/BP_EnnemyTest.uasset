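; BP_EnnemyTest is a test enemy that catches the first-person player on contact.
; When its Hitbox overlaps the first-person character, it shows the UIOnCaught widget and teleports the player to a hardcoded location.
; After a short delay it removes all widgets from the screen, not just the caught message.
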(event OnComponentBeginOverlap(Hitbox)
  (params (OverlappedComponent :type Primitive%20Component%20Object%20Reference) (OtherActor :type Actor%20Object%20Reference) (OtherComp :type Primitive%20Component%20Object%20Reference) (OtherBodyIndex :type Integer) (bFromSweep :type Boolean) (SweepResult :type Hit%20Result%20Structure%20%28by%20ref%29))
  (bind _fpcharacter (CallFunction|GetFirstPersonCharacter))
  (if (== _fpcharacter OtherActor)
    (bind _returnvalue (UserInterface|CreateWidget "/Game/Blueprints/UIOnCaught.UIOnCaught_C"))
    (UserInterface|Viewport|AddtoViewport _returnvalue 0)
    (bind _fpcharacter_2 (CallFunction|GetFirstPersonCharacter))
    (Transformation|SetActorLocationAndRotation _fpcharacter_2 "-170.000000,2420.000000,1192.000000" "0, 0, 0" false true)
    (Utilities|FlowControl|Delay 1.5)
    (Viewport|RemoveAllWidgets)))

(fn ConstructionScript
  (|CallParentFunction))