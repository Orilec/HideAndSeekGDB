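; Bear trap Blueprint that stuns the first-person player when its behaviour is executed.
; While active, ExecuteBehaviour snaps both jaw meshes shut by setting their relative rotations, sets the player's stunned flag and deactivates the trap.
; After a StunDuration delay it clears the stun; nothing here re-arms the trap or reopens the jaws.
; The construction script only calls its parent's.
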(event EventExecuteBehaviour
  (if (Variables|Default|GetIsActive)
    (Transformation|SetRelativeRotation (Variables|Default|GetSM_BearTrap_FirstJaw) "0, 0,-80.000000" false false)
    (Transformation|SetRelativeRotation (Variables|Default|GetSM_BearTrap_SecondJaw) "0, 0,80.000000" false false)
    (bind _fpcharacter (CallFunction|GetFirstPersonCharacter))
    (Variables|/Game/FirstPersonBP/Blueprints/FirstPersonCharacter.FirstPersonCharacter_C|SetPlayerIsStunned _fpcharacter true)
    (Variables|Default|SetIsActive false)
    (Utilities|FlowControl|Delay (Variables|Default|GetStunDuration))
    (bind _fpcharacter_2 (CallFunction|GetFirstPersonCharacter))
    (Variables|/Game/FirstPersonBP/Blueprints/FirstPersonCharacter.FirstPersonCharacter_C|SetPlayerIsStunned _fpcharacter_2 false)))

(fn ConstructionScript
  (|CallParentFunction))