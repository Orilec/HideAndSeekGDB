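; BP_LabyrinthDoor is a labyrinth door with two lock flags that disappears when opened.
; Each unlock event either prints a French "lock opened" message or calls DoorOpen, based on a lock flag.
; Both events clear FirstLock, so UnlockSecondLock always opens the door and SecondLock is never cleared here.
; DoorOpen destroys the Cube component, shows the UIDoorOpened widget, then removes all widgets after a short delay.
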(event Custom|UnlockFirstLock
  (Variables|Default|SetFirstLock false)
  (if (Variables|Default|GetSecondLock)
    (Development|PrintString "Un verrou a été ouvert")
    (else
      (CallFunction|DoorOpen))))

(event Custom|UnlockSecondLock
  (Variables|Default|SetFirstLock false)
  (if (Variables|Default|GetFirstLock)
    (Development|PrintString "Un verrou a été ouvert")
    (else
      (CallFunction|DoorOpen))))

(event Custom|Door%20Open
  (Components|DestroyComponent (Variables|Default|GetCube))
  (bind _returnvalue (UserInterface|CreateWidget "/Game/Blueprints/UIDoorOpened.UIDoorOpened_C"))
  (UserInterface|Viewport|AddtoViewport _returnvalue 0)
  (Utilities|FlowControl|Delay 3.0)
  (Viewport|RemoveAllWidgets))

(fn ConstructionScript)