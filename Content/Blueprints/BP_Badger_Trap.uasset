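; BP_Badger_Trap is a single-use bear-trap-style trap that temporarily changes the first-person character's walk speed.
; When ExecuteBehaviour fires while active, it snaps both jaw meshes to opposing rotations and deactivates itself.
; It sets the character's max walk speed to Speed, waits for Duration, then restores a hardcoded default rather than the previous value.
; The trigger is not in this graph, and nothing here re-arms the trap.
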(event EventExecuteBehaviour
  (if (Variables|Default|GetIsActive)
    (Transformation|SetRelativeRotation (Variables|Default|GetSM_BearTrap_FirstJaw) "0, 0,-80.000000" false false)
    (Transformation|SetRelativeRotation (Variables|Default|GetSM_BearTrap_SecondJaw) "0, 0,80.000000" false false)
    (Variables|Default|SetIsActive false)
    (bind _fpcharacter (CallFunction|GetFirstPersonCharacter))
    (Variables|/Script/Engine.CharacterMovementComponent|SetMaxWalkSpeed (Variables|/Script/Engine.Character|GetCharacterMovement _fpcharacter) (Variables|Default|GetSpeed))
    (Utilities|FlowControl|Delay (Variables|Default|GetDuration))
    (bind _fpcharacter_2 (CallFunction|GetFirstPersonCharacter))
    (Variables|/Script/Engine.CharacterMovementComponent|SetMaxWalkSpeed (Variables|/Script/Engine.Character|GetCharacterMovement _fpcharacter_2) 6e+02)))

(fn ConstructionScript
  (|CallParentFunction))