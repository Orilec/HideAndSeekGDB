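; BP_Door is a door that toggles open and closed each time its ExecuteBehaviour event fires.
; A FlipFlop on that event sets IsOpen, which Tick reads to pick a target yaw: a quarter turn when open, zero when closed.
; Tick nudges the door mesh's relative yaw toward that target in small fixed steps, using a Delay loop paced by PorteVitesse until within tolerance.
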(event EventTick
  (params (DeltaSeconds :type Float%20%28single-precision%29))
  (bind _sm_porte_porte_porte (Variables|Default|GetSM_Porte_Porte_Porte))
  (bind _sm_porte_porte_porte_2 (Variables|Default|GetSM_Porte_Porte_Porte))
  (bind _relativerotation (Variables|/Script/Engine.SceneComponent|GetRelativeRotation _sm_porte_porte_porte_2))
  (bind _relativerotation_2 (Variables|/Script/Engine.SceneComponent|GetRelativeRotation _sm_porte_porte_porte))
  (bind (_roll _pitch _yaw) (Math|Rotator|BreakRotator _relativerotation))
  (bind (_roll_2 _pitch_2 _yaw_2) (Math|Rotator|BreakRotator _relativerotation_2))
  (if (Variables|Default|GetIsOpen) :!label _label
    (if (Utilities|Enum|NotEqual(Enum) (Variables|/Script/Engine.SceneComponent|GetRelativeRotation (Variables|Default|GetSM_Porte_Porte_Porte)) "0,90.000000, 0" 0.5)
      (Utilities|FlowControl|Delay (Variables|Default|GetPorteVitesse))
      (Utilities|FlowControl|Sequence
        (:then_0
          (Transformation|SetRelativeRotation _sm_porte_porte_porte (Math|Rotator|MakeRotator _roll_2 _pitch_2 (+ _yaw_2 0.2)) false false))
        (:then_1
          (goto _label))))
    (elif (Utilities|Enum|NotEqual(Enum) (Variables|/Script/Engine.SceneComponent|GetRelativeRotation (Variables|Default|GetSM_Porte_Porte_Porte)) "0,0.000000, 0" 0.5)
      (Utilities|FlowControl|Delay (Variables|Default|GetPorteVitesse))
      (Utilities|FlowControl|Sequence
        (:then_0
          (Transformation|SetRelativeRotation _sm_porte_porte_porte_2 (Math|Rotator|MakeRotator _roll _pitch (+ _yaw -0.2)) false false))
        (:then_1
          (goto _label))))))

(event EventExecuteBehaviour
  (Utilities|FlowControl|FlipFlop
    (:A
      (Variables|Default|SetIsOpen true))
    (:B
      (Variables|Default|SetIsOpen false))))

(fn ConstructionScript
  (|CallParentFunction))