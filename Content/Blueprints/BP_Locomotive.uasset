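; BP_Locomotive is a locomotive that travels a looping route of waypoints stored in the TableauPosition data table.
; It starts at PositionInitiale, then every Tick looks up the row for its current index, reissues AI MoveTo and yaws its root toward that point.
; On arrival, the index advances or wraps to zero after PositionMax, with a short delayed flag preventing repeated increments.
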(event Custom|PositionJustChanged
  (Utilities|FlowControl|Delay 0.2)
  (Variables|Default|SetPositionCanChange true))

(event EventBeginPlay
  (Transformation|SetRelativeLocation (Variables|Default|GetDefaultSceneRoot self) (Variables|Default|GetPositionInitiale) false true))

(event EventTick
  (params (DeltaSeconds :type Float%20%28single-precision%29))
  (|CallParentFunction DeltaSeconds)
  (bind _returnvalue (Utilities|GetDataTableRow (Variables|Default|GetTableau_Position) (Utilities|String|StringToName (Utilities|String|ToString(Integer) (Variables|Default|GetPosition))))
    (:then
      (AI|AIMoveTo (Class|PawnMovementComponent|GetPawnOwner (Variables|Default|GetFloatingPawnMovement)) (Utilities|Struct|BreakStruct_PositionLocomotive _returnvalue) 0 0.001 false
        (:then
          (Transformation|SetRelativeRotation (Variables|Default|GetDefaultSceneRoot) (Math|Rotator|MakeRotator 0.0 0.0 (.Yaw (Math|Rotator|BreakRotator (Math|Conversions|RotationFromXVector (- (Utilities|Struct|BreakStruct_PositionLocomotive _returnvalue) (Transformation|GetWorldLocation (Variables|Default|GetDefaultSceneRoot))))))) false false))
        (:OnSuccess
          (if (Variables|Default|GetPositionCanChange)
            (if (== (Variables|Default|GetPositionMax) (Variables|Default|GetPosition))
              (Variables|Default|SetPosition 0)
              (else
                (Variables|Default|SetPosition (+ (Variables|Default|GetPosition) 1))))
            (Variables|Default|SetPositionCanChange false)
            (CallFunction|PositionJustChanged)))))))

(fn ConstructionScript
  (|CallParentFunction))