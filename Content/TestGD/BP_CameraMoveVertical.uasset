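; Security camera that sweeps back and forth, watches for targets and alerts a linked enemy.
; A timeline ping-pongs the Cam's roll across a per-instance span and speed, while construction applies per-instance vision angle and distance to SCPawnSensing.
; Tick polls that component: while seeing, the actor turns toward the player pawn.
; DoOnce-gated seen/unseen events stop or resume the sweep, restore initial rotation and notify LinkedEnemy.
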(event Custom|OnSeen
  (CallFunction|CameraAnimationStop)
  (Default|OnSeen (Variables|Default|GetLinkedEnemy)))

(event Custom|OnUnseen
  (CallFunction|CameraAnimationForward)
  (Default|OnUnseen (Variables|Default|GetLinkedEnemy)))

(event Custom|Camera_Animation_Stop
  (bind _instance_vision_span (Variables|Default|GetInstance_Vision_Span))
  (bind (_direction _alpha) (Timeline|Camera_Rotation_Animation Stop)
    (:Update
      (Variables|Default|SetCamera_Rotation_Animation_Direction _direction)
      (Transformation|SetRelativeRotation (Variables|Default|GetCam) (Math|Rotator|MakeRotator (Math|Float|Lerp (.x _instance_vision_span) (.y _instance_vision_span) _alpha) 0.0 0.0) false false))
    (:Finished
      (if (Utilities|Enum|Equal(Enum) (Variables|Default|GetCamera_Rotation_Animation_Direction) "Forward")
        (CallFunction|CameraAnimationReverse)
        (else
          (CallFunction|CameraAnimationForward))))))

(event Custom|Camera_Animation_Forward
  (bind _instance_vision_span (Variables|Default|GetInstance_Vision_Span))
  (Components|Timeline|SetPlayRate (Variables|Default|GetCamera_Rotation_Animation) (Variables|Default|GetInstance_Rotation_Speed))
  (bind (_direction _alpha) (Timeline|Camera_Rotation_Animation Play)
    (:Update
      (Variables|Default|SetCamera_Rotation_Animation_Direction _direction)
      (Transformation|SetRelativeRotation (Variables|Default|GetCam) (Math|Rotator|MakeRotator (Math|Float|Lerp (.x _instance_vision_span) (.y _instance_vision_span) _alpha) 0.0 0.0) false false))
    (:Finished
      (if (Utilities|Enum|Equal(Enum) (Variables|Default|GetCamera_Rotation_Animation_Direction) "Forward")
        (CallFunction|CameraAnimationReverse)
        (else
          (CallFunction|CameraAnimationForward))))))

(event Custom|Camera_Animation_Reverse
  (bind _instance_vision_span (Variables|Default|GetInstance_Vision_Span))
  (bind (_direction _alpha) (Timeline|Camera_Rotation_Animation Reverse)
    (:Update
      (Variables|Default|SetCamera_Rotation_Animation_Direction _direction)
      (Transformation|SetRelativeRotation (Variables|Default|GetCam) (Math|Rotator|MakeRotator (Math|Float|Lerp (.x _instance_vision_span) (.y _instance_vision_span) _alpha) 0.0 0.0) false false))
    (:Finished
      (if (Utilities|Enum|Equal(Enum) (Variables|Default|GetCamera_Rotation_Animation_Direction) "Forward")
        (CallFunction|CameraAnimationReverse)
        (else
          (CallFunction|CameraAnimationForward))))))

(event EventTick
  (params (DeltaSeconds :type Float%20%28single-precision%29))
  ;[1 1 1] Vision Event fired from Vision component data
  (if (Variables|/Game/TestGD/SC_PawnSensing.SC_PawnSensing_C|GetVision_SeeingSomething? (Variables|Default|GetSC_PawnSensing))
    (|lookat
      (:then2
        (Utilities|FlowControl|DoOnce false :!label _label
          (:Completed
            (CallFunction|OnSeen)
            (goto _label_2 Reset)))))
    (else
      (Utilities|FlowControl|DoOnce false :!label _label_2
        (:Completed
          (CallFunction|OnUnseen)
          (Transformation|SetActorRotation (Variables|Default|GetInitial_Rotation))
          (goto _label Reset))))))

(event EventBeginPlay
  (if (not false)
    (CallFunction|CameraAnimationForward)))

(fn ConstructionScript
  (Variables|/Game/TestGD/SC_PawnSensing.SC_PawnSensing_C|SetComponent_Vision_Angle (Variables|Default|GetSC_PawnSensing) (Variables|Default|GetInstance_Vision_Angle))
  (Variables|/Game/TestGD/SC_PawnSensing.SC_PawnSensing_C|SetComponent_Vision_Length (Variables|Default|GetSC_PawnSensing) (Variables|Default|GetInstance_Vision_Distance)))