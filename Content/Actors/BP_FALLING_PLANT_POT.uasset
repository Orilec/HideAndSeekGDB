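; Falling plant pot trap actor that fires on collider overlap, or on an interaction message from an actor overlapping the collider.
; The overlap path runs once via DoOnce, while ExecuteBehaviour bypasses that gate.
; It prints debug text, adds one movement input to the player pawn and destroys itself.
; The intended three-second control change is only printed, and its delayed restore follows DestroyActor.
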(event OnComponentBeginOverlap(Collider)
  (params (OverlappedComponent :type Primitive%20Component%20Object%20Reference) (OtherActor :type Actor%20Object%20Reference) (OtherComp :type Primitive%20Component%20Object%20Reference) (OtherBodyIndex :type Integer) (bFromSweep :type Boolean) (SweepResult :type Hit%20Result%20Structure%20%28by%20ref%29))
  (bind _returnvalue (Game|Player|GetPlayerPawn 0))
  (Utilities|FlowControl|DoOnce false
    (:Completed
      (Development|PrintString "The trap is detected. Aeiou.")
      (Pawn|Input|AddMovementInput _returnvalue "-1.000000,-1.000000,-1.000000" -1.0 false)
      (Actor|DestroyActor)
      (Development|PrintString "Player controls are changed")
      (Utilities|FlowControl|Delay 3.0)
      (Pawn|Input|AddMovementInput _returnvalue "1.000000,1.000000,1.000000" 1.0 false)
      (Development|PrintString "Player controls are back to default"))))

(event Custom|ExecuteBehaviour
  (bind _returnvalue (Game|Player|GetPlayerPawn 0))
  (Development|PrintString "The trap is detected. Aeiou.")
  (Pawn|Input|AddMovementInput _returnvalue "-1.000000,-1.000000,-1.000000" -1.0 false)
  (Actor|DestroyActor)
  (Development|PrintString "Player controls are changed")
  (Utilities|FlowControl|Delay 3.0)
  (Pawn|Input|AddMovementInput _returnvalue "1.000000,1.000000,1.000000" 1.0 false)
  (Development|PrintString "Player controls are back to default"))

(event EventInteractionMessage
  (params (Sender :type Actor%20Object%20Reference))
  (if (Collision|IsOverlappingActor (Variables|Default|GetCollider) Sender :!class /Script/Engine.PrimitiveComponent)
    (CallFunction|ExecuteBehaviour)))

(fn ConstructionScript)