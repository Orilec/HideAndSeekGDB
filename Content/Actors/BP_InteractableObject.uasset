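; BP_InteractableObject is an interactable actor that responds to an overlap message from the player.
; OverlappedMessage casts the sender to ThirdPersonCharacter and stores it as Player.
; When NeedPlayerVision is set, it calls CheckLookedAt to compare the player's LookedAtActor with itself, then calls ExecuteBehaviour, a debug-print placeholder.
; The look check returns no result, so it does not gate the behaviour, and nothing runs when the flag is off.
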(event EventOverlappedMessage
  (params (Sender :type Actor%20Object%20Reference))
  (Utilities|FlowControl|Sequence
    (:then_0
      (bind _asthird_person_character (Utilities|Casting|CastToThirdPersonCharacter Sender))
      (Variables|Default|SetPlayer _asthird_person_character))
    (:then_1
      (if (Variables|Default|GetNeedPlayerVision)
        (|CheckLookedAt)
        (CallFunction|ExecuteBehaviour)))))

(fn ConstructionScript)

(fn ExecuteBehaviour
  (Development|PrintString "Behaviour executed"))